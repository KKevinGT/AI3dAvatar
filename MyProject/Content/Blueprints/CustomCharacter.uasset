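; Customizable character Blueprint that supports outfit changes through modular skeletal meshes for clothing and accessory slots, all following the Head mesh's pose.
; UpdatePlayerCloth maps a category to its component and returns it.
; A full outfit clears the separate pieces, while other categories clear the outfit and restore default top, bottom and shoes where empty, swapping body material and All1 visibility.
; GetMat steps through a material array using a wrapping counter.
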(fn ConstructionScript
  (Class|SkinnedMeshComponent|SetMasterPoseComponent (Variables|Default|Getxiazhuang) (Variables|Default|GetHead) false))

(fn GetMat
  (params (Mat :type Array%20of%20Material%20Instance%20Object%20References))
  (Math|Integer|CompareInt (Variables|Default|GetCount) (- (Utilities|Array|Length Mat) 1)
    (:>
      (Variables|Default|SetCount 0 :!label _label))
    (:==
      (goto _label))
    (:<
      (bind _result (Math|Integer|IncrementInt (Variables|Default|GetCount))
        (:%20%20
          _))))
  (return (Utilities|Array|Get(acopy) Mat _result)))

(fn UpdatePlayerCloth
  (params (NewParam :type E_ItemClothType%20Enum :default "NewEnumerator1"))
  (bind _xiazhuang (Variables|Default|Getxiazhuang))
  (bind _xiezi (Variables|Default|Getxiezi))
  (bind _all (Variables|Default|GetAll))
  (bind _shangyi (Variables|Default|Getshangyi))
  (switch Utilities|FlowControl|Switch|SwitchonE_ItemClothType NewParam
    (:NewEnumerator1
      (Variables|Default|SetTemp (Variables|Default|Getshangyi))
      (Utilities|FlowControl|Sequence :!label _label
        (:then_0
          (Utilities|IsValid (Variables|/Script/Engine.SkinnedMeshComponent|GetSkeletalMesh _shangyi)
            (:Is%20Not%20Valid
              (Class|SkinnedMeshComponent|SetSkeletalMesh _shangyi "/Game/Model/基础装/tixu.tixu" true))))
        (:then_1
          (Utilities|IsValid (Variables|/Script/Engine.SkinnedMeshComponent|GetSkeletalMesh _xiazhuang)
            (:Is%20Not%20Valid
              (Class|SkinnedMeshComponent|SetSkeletalMesh _xiazhuang "/Game/Model/基础装/baizhehun.baizhehun" true))))
        (:then_2
          (Utilities|IsValid (Variables|/Script/Engine.SkinnedMeshComponent|GetSkeletalMesh _xiezi)
            (:Is%20Not%20Valid
              (Class|SkinnedMeshComponent|SetSkeletalMesh _xiezi "/Game/Model/基础装/xiezi.xiezi" true))))
        (:then_3
          (Utilities|IsValid (Variables|/Script/Engine.SkinnedMeshComponent|GetSkeletalMesh _all)
            (:Is%20Valid
              (Class|SkinnedMeshComponent|SetSkeletalMesh _all 0 true)
              (Rendering|SetVisibility (Variables|Default|GetAll1) false true)
              (Rendering|Material|SetMaterial (Variables|Default|GetHead) 1 "/Game/Model/人物/M_body2.M_body2"))))
        (:then_4
          (return (Variables|Default|GetTemp)))))
    (:NewEnumerator2
      (Variables|Default|SetTemp (Variables|Default|Getxiazhuang))
      (goto _label))
    (:NewEnumerator3
      (Variables|Default|SetTemp (Variables|Default|Getxiezi))
      (goto _label))
    (:NewEnumerator0
      (Variables|Default|SetTemp (Variables|Default|GetAll))
      (Class|SkinnedMeshComponent|SetSkeletalMesh (Variables|Default|Getshangyi) 0 true)
      (Rendering|Material|SetMaterial (Variables|Default|GetHead) 1 "/Game/Model/人物/M_Body.M_Body")
      (Rendering|SetVisibility (Variables|Default|GetAll1) true true)
      (return (Variables|Default|GetTemp)))
    (:NewEnumerator4
      (Variables|Default|SetTemp (Variables|Default|Getfashi))
      (goto _label))
    (:NewEnumerator7
      (Variables|Default|SetTemp (Variables|Default|Geterhuan))
      (goto _label))
    (:NewEnumerator5
      (Variables|Default|SetTemp (Variables|Default|Getxianglian))
      (goto _label))
    (:NewEnumerator6
      (Variables|Default|SetTemp (Variables|Default|Getshoushi))
      (goto _label))))