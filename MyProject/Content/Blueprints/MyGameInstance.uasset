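; Game instance for a character clothing customization feature, holding saved parts, clothing data and animation data.
; Clothing and animation rows load from DataTables by numeric row names, and animation names fill a combo box in MainView.
; Type buttons show or hide inventory slots by clothing type.
; Changing clothes applies the selected item's skeletal mesh and materials to the given body part.
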(event Custom|StoreSavedParts
  (params (SavedParts :type S%20Saved%20Parts%20Structure))
  (Variables|Default|SetSavedParts SavedParts))

(event Custom|InitAnimatorWeight
  (bind _mainview (Variables|Default|GetMainView))
  (bind _allanimatorlist (Variables|Default|GetAllAnimatorList))
  (bind _comboboxstring_0 (Variables|/Game/Widget/W_MainView.W_MainView_C|GetComboBoxString_0 _mainview))
  (CallFunction|OnInitAnimatorList)
  (for _index (range 1 (Variables|Default|GetAnimationNumber))
    (Class|ComboBoxString|AddOption _comboboxstring_0 (.Name (Utilities|Struct|Breaks_AnimatorItem (Utilities|Array|Get(acopy) _allanimatorlist (- _index 1))))))
  (Class|ComboBoxString|SetSelectedOption _comboboxstring_0 (.Name (Utilities|Struct|Breaks_AnimatorItem (Utilities|Array|Get(acopy) _allanimatorlist)))))

(fn GetSavedParts
  (return (Variables|Default|GetSavedParts)))

(fn ShowCurrentTypeCloth
  (bind _mainview (Variables|Default|GetMainView))
  (for (_array_element _array_index) (Variables|/Game/Blueprints/BP_Inventory.BP_Inventory_C|GetSlots (Variables|/Game/Widget/W_MainView.W_MainView_C|GetInventory _mainview))
    (Default|OnSetCurrentSHoworHide (Utilities|Array|Get(acopy) (Variables|/Game/Widget/W_MainView.W_MainView_C|GetW_Slots _mainview) _array_index) (Utilities|Enum|Equal(Enum) (.Type (Utilities|Struct|BreakS_Slot _array_element)) (Variables|Default|GetCurrentClothType)))))

(fn OnClickTypeButton
  (params (Type :type E_ItemClothType%20Enum :default "NewEnumerator1"))
  (Variables|Default|SetCurrentClothType Type)
  (CallFunction|ShowCurrentTypeCloth)
  (Default|OnResetGridePanle (Variables|Default|GetMainView)))

(fn OnInitClothList
  (bind _clothscount (Variables|Default|GetClothsCount))
  (while (> _clothscount 0)
    (bind _returnvalue (Utilities|GetDataTableRow (Variables|Default|GetClothDataTable) (Utilities|String|StringToName (Utilities|String|ToString(Integer) _clothscount)))
      (:then
        (Utilities|Array|Add (Variables|Default|GetAllClothItem) _returnvalue)
        (Math|Integer|DecrementInt _clothscount)))))

(fn OnSetModelSkelenMeshbySlot
  (params (index :type Integer))
  (bind _allclothitem (Variables|Default|GetAllClothItem))
  (bind _output (Utilities|Array|Get(acopy) _allclothitem index))
  (bind (_id _name _itemtype _model _material _slotimage) (Utilities|Struct|BreakS_ClothItem _output))
  (return _itemtype _slotimage))

(fn OnChangeClothFunction
  (params (Part :type Skinned%20Mesh%20Component%20Object%20Reference) (Index :type Integer))
  (bind _allclothitem (Variables|Default|GetAllClothItem))
  (bind _output (Utilities|Array|Get(acopy) _allclothitem Index))
  (bind (_id _name _itemtype _model _material) (Utilities|Struct|BreakS_ClothItem _output))
  (for (_ _array_index) _model
    (Class|SkinnedMeshComponent|SetSkeletalMesh Part (Utilities|Array|Get(acopy) _model _array_index) true)
    (for (_array_element _array_index_2) _material
      (Rendering|Material|SetMaterial Part _array_index_2 _array_element))))

(fn OnInitAnimatorList
  (for _index (range 1 (Variables|Default|GetAnimationNumber))
    (bind _returnvalue (Utilities|GetDataTableRow (Variables|Default|GetAnimatorDataTable) (Utilities|String|StringToName (Utilities|String|ToString(Integer) _index)))
      (:then
        (Utilities|Array|Add (Variables|Default|GetAllAnimatorList) _returnvalue)))))