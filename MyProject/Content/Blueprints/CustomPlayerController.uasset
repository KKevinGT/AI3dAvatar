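; Player controller for a character-customization screen driven by a UI widget.
; On BeginPlay it creates the main view, spawns an inventory actor, links both to the game instance, fills clothing slots, selects a default type and switches to UI-only input with a visible cursor.
; It caches the CustomCharacter found in the level and forwards animator-type changes to the ABP_DXX anim instance on that character's head mesh.
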(event Custom|OnChangeAnimatorType
  (params (CurrentAnimatorType :type E_AnimatorType%20Enum :default "NewEnumerator0"))
  (bind _customchar (Variables|Default|GetCustomChar))
  (Utilities|IsValid _customchar
    (:Is%20Valid
      (bind _asabp_dxx (Utilities|Casting|CastToABP_DXX (Components|SkeletalMesh|GetAnimInstance (Variables|/Game/Blueprints/CustomCharacter.CustomCharacter_C|GetHead _customchar))))
      (Variables|/Game/Model/人物/ABP_DXX.ABP_DXX_C|SetCurrentAnimatorType _asabp_dxx CurrentAnimatorType))))

(event EventBeginPlay
  (bind _asmy_game_instance (Utilities|Casting|CastToMyGameInstance (Game|GetGameInstance)))
  (bind _output_get (Variables|Default|SetGameInstance _asmy_game_instance))
  (bind _returnvalue (UserInterface|CreateWidget "/Game/Widget/W_MainView.W_MainView_C" 0 0))
  (Variables|/Game/Blueprints/MyGameInstance.MyGameInstance_C|SetMainView _output_get _returnvalue)
  (bind _output_get_2 (Variables|Default|SetW_Mainwidget _returnvalue))
  (UserInterface|Viewport|AddtoViewport _output_get_2 0)
  (Variables|/Game/Blueprints/MyGameInstance.MyGameInstance_C|SetMainView (Variables|Default|GetGameInstance) _returnvalue)
  (bind _returnvalue_2 (Game|SpawnActorfromClass "/Game/Blueprints/BP_Inventory.BP_Inventory_C" (Math|Transform|MakeTransform "0, 0, 0" "0, 0, 0" "1,1,1") "AlwaysSpawn" 0 0))
  (bind _output_get_3 (Variables|Default|SetInventoryRef _returnvalue_2))
  (Variables|/Game/Widget/W_MainView.W_MainView_C|SetInventory _returnvalue _output_get_3)
  (Default|OnInitClothList (Variables|Default|GetGameInstance))
  (Default|InitSlots _output_get_2 (Variables|/Game/Blueprints/MyGameInstance.MyGameInstance_C|GetAllClothItem (Variables|Default|GetGameInstance)))
  (Default|OnClickTypeButton (Variables|Default|GetGameInstance) "NewEnumerator1")
  (Input|SetInputModeUIOnly self (Variables|Default|GetW_Mainwidget) "DoNotLock")
  (Variables|Default|SetbShowMouseCursor true)
  (bind _outactors (Actor|GetAllActorsOfClass "/Game/Blueprints/CustomCharacter.CustomCharacter_C"))
  (for _array_element _outactors
    (Variables|Default|SetCustomChar _array_element)))

(fn ConstructionScript)